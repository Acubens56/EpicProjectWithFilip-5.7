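; Spline actor whose construction script populates a spline with copies of a chosen mesh, with collision enabled.
; For each point segment it adds a scaled spline mesh without assigning a mesh, then repeats a full-length placement pass.
; That pass either places rotated copies at spaced intervals or bends end-to-end pieces by mesh length, clamping tangents via GetLocationAndTangent.
; Up-vector and debug arrow logic is disconnected.
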(event EventBeginPlay)

(event Collision|EventActorBeginOverlap
  (params (OtherActor :type Actor%20Object%20Reference)))

(event EventTick
  (params (DeltaSeconds :type Float%20%28single-precision%29)))

(fn ConstructionScript
  (bind _spline (Variables|Default|GetSpline))
  (bind _spline_2 (Variables|Default|GetSpline))
  (bind _spline_3 (Variables|Default|GetSpline))
  (bind _spline_mesh (Variables|Default|GetSpline%20Mesh))
  (bind _returnvalue (StaticMesh|GetBoundingBox _spline_mesh))
  (bind _returnvalue_2 (- (.max _returnvalue) (.min _returnvalue)))
  (for _index (range 0 (- (Spline|GetNumberOfSplinePoints (Variables|Default|GetSpline)) 2))
    (bind _returnvalue_3 (AddComponent|AddSplineMeshComponent false))
    (SplineMesh|SetForwardAxis _returnvalue_3 "Z" true)
    (SplineMesh|SetStartScale _returnvalue_3 (Math|Conversions|ToVector2D(Vector) (Spline|GetScaleatSplinePoint _spline_2 _index)) true :!class /Script/Engine.SplineMeshComponent)
    (SplineMesh|SetEndScale _returnvalue_3 (Math|Conversions|ToVector2D(Vector) (Spline|GetScaleatSplinePoint _spline_2 (+ _index 1))) true :!class /Script/Engine.SplineMeshComponent)
    (SplineMesh|SetStartandEnd _returnvalue_3 (.Location (Spline|GetLocationandTangentatSplinePoint _spline _index "Local")) (.Tangent (Spline|GetLocationandTangentatSplinePoint _spline _index "Local")) (.Location (Spline|GetLocationandTangentatSplinePoint _spline (+ _index 1) "Local")) (.Tangent (Spline|GetLocationandTangentatSplinePoint _spline (+ _index 1) "Local")) true :!class /Script/Engine.SplineMeshComponent)
    (if (Utilities|Enum|Equal(Enum) (Variables|Default|GetIn%20Forward%20Axis) "X")
      (Variables|Default|SetMesh%20Length (.x _returnvalue_2))
      (elif (Utilities|Enum|Equal(Enum) (Variables|Default|GetIn%20Forward%20Axis) "Y")
        (Variables|Default|SetMesh%20Length (.y _returnvalue_2))
        (else
          (Variables|Default|SetMesh%20Length (.z _returnvalue_2)))))
    (if (Variables|Default|GetSpace%20Meshes)
      (Variables|Default|SetSectionLength (+ (Variables|Default|GetSpacing) (Variables|Default|GetMesh%20Length)))
      (for _index_2 (range 0 (Math|Float|Truncate (/ (Spline|GetSplineLength (Variables|Default|GetSpline)) (Variables|Default|GetSectionLength))))
        (Variables|Default|SetIndex _index_2)
        (bind _returnvalue_4 (AddComponent|AddSplineMeshComponent false (Math|Transform|MakeTransform (Spline|GetLocationatDistanceAlongSpline _spline_3 (* (Variables|Default|GetIndex) (Variables|Default|GetSectionLength)) "Local") (Math|Rotator|CombineRotators (Variables|Default|GetMeshRotation) (Spline|GetRotationatDistanceAlongSpline _spline_3 (* (Variables|Default|GetIndex) (Variables|Default|GetSectionLength)) "Local")))))
        (Components|StaticMesh|SetStaticMesh _returnvalue_4 (Variables|Default|GetSpline%20Mesh))
        (Collision|SetCollisionEnabled _returnvalue_4 "QueryAndPhysics")
        (SplineMesh|SetForwardAxis _returnvalue_4 (Variables|Default|GetIn%20Forward%20Axis) true))
      (else
        (for _index_3 (range 0 (Math|Float|Truncate (/ (Spline|GetSplineLength (Variables|Default|GetSpline)) (Variables|Default|GetMesh%20Length))))
          (Variables|Default|SetIndex _index_3)
          (bind _returnvalue_5 (AddComponent|AddSplineMeshComponent false))
          (Components|StaticMesh|SetStaticMesh _returnvalue_5 (Variables|Default|GetSpline%20Mesh))
          (Collision|SetCollisionEnabled _returnvalue_5 "QueryAndPhysics")
          (SplineMesh|SetForwardAxis _returnvalue_5 (Variables|Default|GetIn%20Forward%20Axis) true)
          (bind (_returnvalue_6 _returnvalue2) (CallFunction|GetLocationandTangent (Variables|Default|GetIndex)))
          (bind (_returnvalue_7 _returnvalue2_2) (CallFunction|GetLocationandTangent (+ (Variables|Default|GetIndex) 1)))
          (SplineMesh|SetStartandEnd _returnvalue_5 _returnvalue_6 _returnvalue2 _returnvalue_7 _returnvalue2_2 true :!class /Script/Engine.SplineMeshComponent))))))

(fn GetLocationandTangent
  (params (A :type Integer))
  (bind _spline (Variables|Default|GetSpline))
  (bind _mesh_length (Variables|Default|GetMesh%20Length))
  (bind _returnvalue (* A _mesh_length))
  (return (Spline|GetLocationatDistanceAlongSpline _spline _returnvalue "Local") (Math|Vector|ClampVectorSize (Spline|GetTangentatDistanceAlongSpline _spline _returnvalue "Local") 0.0 (Variables|Default|GetMesh%20Length))))